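; BP_CoinDoor is a door that opens, by destroying itself, once every coin in its CoinsLeft list has been collected.
; Each tick it checks whether the player overlaps its Box and the IA_OpenDoor input is pressed, then whether the list is empty.
; RemoveCoins takes a coin out of that list, and input is enabled for player 0 on BeginPlay.
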(event `self.ReceiveBeginPlay`
  (`self.CreateInputComponent` "/Script/EnhancedInput.EnhancedInputComponent")
  (`self.EnableInput` (`GameplayStatics.GetPlayerController` 0)))

(event `self.ReceiveTick`
  (params (DeltaSeconds :type "Float (single-precision)"))
  (if (`PrimitiveComponent.IsOverlappingActor` (`self.Box`) (`GameplayStatics.GetPlayerCharacter` 0))
    (if (`|GetInputActionValue`)
      (if (== (`BlueprintSetLibrary.Set_Length` (`self.CoinsLeft`)) 0)
        (`self.K2_DestroyActor`)))))

(fn `RemoveCoins`
  (params (Coin :type "/Game/Blueprints/Coins/BP_Coins Object Reference (by ref)"))
  (`BlueprintSetLibrary.Set_Remove` (`self.CoinsLeft`) Coin))

(fn `UserConstructionScript`)