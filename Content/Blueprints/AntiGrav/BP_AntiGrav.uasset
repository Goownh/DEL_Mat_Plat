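; BP_AntiGrav is a trigger actor that changes the gravity of a third-person character that touches it.
; When something begins overlapping its Box and the cooldown has expired, it casts to BP_ThirdPersonCharacter and calls ChangeGrav with a fixed negative vector.
; A successful trigger stores a game-time timestamp two seconds ahead, blocking retriggers until then without using timers or Tick.
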(event `self.ReceiveBeginPlay`)

(event `self.Box.OnComponentBeginOverlap`
  (params (OverlappedComponent :type "PrimitiveComponent Object Reference") (OtherActor :type "Actor Object Reference") (OtherComp :type "PrimitiveComponent Object Reference") (OtherBodyIndex :type Integer) (bFromSweep :type Boolean) (SweepResult :type "HitResult Structure (by ref)"))
  (`/Engine/EditorBlueprintResources/StandardMacros.CompareFloat` (`self.AntiGravCooldown`) (`KismetSystemLibrary.GetGameTimeInSeconds`)
    (:`<`
      (bind _asbp_third_person_character (cast `/Game/Blueprints/ThirdPerson/BP_ThirdPersonCharacter` OtherActor))
      (`/Game/Blueprints/ThirdPerson/BP_ThirdPersonCharacter.ChangeGrav` _asbp_third_person_character (-100.0 -100.0 -100.0))
      (set `self.AntiGravCooldown` (+ (`KismetSystemLibrary.GetGameTimeInSeconds`) 2.0)))))

(event `self.ReceiveTick`
  (params (DeltaSeconds :type "Float (single-precision)")))

(fn `UserConstructionScript`)